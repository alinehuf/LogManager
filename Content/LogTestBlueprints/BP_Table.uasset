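; BP_Table is a table actor that appears or disappears based on the experiment (XP) setting.
; CheckShowHide reads the config info message from the game mode and shows the table only if it succeeded and its setting matches WantedSetting.
; Show and Hide toggle mesh visibility and box collision.
; Both set the nav modifier to the default area class, so that class is identical in either state.
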(event `CheckShowHide`
  ;[0.9517 0.2445 1] Show/Hide table given XP Setting
  (bind (_userid _setting _success) (message `/Game/LogTestBlueprints/I_CanLog.GetConfigInfos` (`GameplayStatics.GetGameMode`)))
  (if (and (== (`self.WantedSetting`) _setting) _success)
    (`self.Show`)
    (else
      (`self.Hide`))))

(event `Hide`
  ;[0.9517 0.2445 1] Show/Hide table given XP Setting
  (`SceneComponent.SetHiddenInGame` (`self.StaticMesh`) true false)
  (`PrimitiveComponent.SetCollisionEnabled` (`self.Box`) "NoCollision")
  (`NavModifierComponent.SetAreaClass` (`self.NavModifier`) "/Script/NavigationSystem.NavArea_Default"))

(event `Show`
  ;[0.9517 0.2445 1] Show/Hide table given XP Setting
  (`SceneComponent.SetHiddenInGame` (`self.StaticMesh`) false false)
  (`PrimitiveComponent.SetCollisionEnabled` (`self.Box`) "QueryAndPhysics")
  (`NavModifierComponent.SetAreaClass` (`self.NavModifier`) "/Script/NavigationSystem.NavArea_Default"))

(fn `UserConstructionScript`)